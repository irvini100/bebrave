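; Custom player controller that toggles pausing and shows or hides a pause menu widget.
; On BeginPlay it caches the GI_GameManager game instance, creates the menu widget and binds to the manager's game state change event.
; The Pause input switches the manager between PLAYING and PAUSED and sets game pause.
; The state change handler adds the menu on entering PAUSED and removes it on leaving.
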(event `self.ReceiveBeginPlay`
  (set `self.Game Manager` (cast `/Game/GI_GameManager` (`GameplayStatics.GetGameInstance`) :!pure true))
  (bind _returnvalue (`|CreateWidget` "/Game/PauseMenu.PauseMenu_C"))
  (set `self.PauseMenu` _returnvalue)
  (add `/Game/GI_GameManager.EventGameStateChanged` (`self.Game Manager`) (delegate `HandleGameStateChange`)))

(event `InputAction|Pause` :paused true
  (params (Key :type "Key Structure"))
  (:`Pressed`
    (switch `/Game/EGameStates` (`/Game/GI_GameManager.CurrentState` (`self.Game Manager`))
      (:`NewEnumerator0`
        (`/Game/GI_GameManager.ChangeState` (`self.Game Manager`) "NewEnumerator1")
        (`GameplayStatics.SetGamePaused` true))
      (:`NewEnumerator1`
        (`/Game/GI_GameManager.ChangeState` (`self.Game Manager`) "NewEnumerator0")
        (`GameplayStatics.SetGamePaused` false)))))

(event `HandleGameStateChange`
  (params (PreviousState :type "/Game/EGameStates Enum" :default "NewEnumerator0") (NewState :type "/Game/EGameStates Enum" :default "NewEnumerator0"))
  (`|ExecutionSequence`
    (:`then_0`
      (switch `/Game/EGameStates` NewState
        (:`NewEnumerator1`
          (`UserWidget.AddToViewport` (`self.PauseMenu`) 0))))
    (:`then_1`
      (switch `/Game/EGameStates` PreviousState
        (:`NewEnumerator1`
          (`Widget.RemoveFromParent` (`self.PauseMenu`)))))))

(fn `UserConstructionScript`)